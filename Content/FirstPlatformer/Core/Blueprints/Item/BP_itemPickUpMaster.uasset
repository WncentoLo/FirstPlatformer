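; Master item pickup actor for the platformer, meant as a base for specific items.
; The interface Interacted event calls an empty Pickup event for children to implement, prints a debug string, then destroys the actor.
; Box overlap events are empty; disconnected leftover nodes would cache the player character, toggle input and show or hide the TextRender prompt.
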(event OnComponentBeginOverlap(Box)
  (params (OverlappedComponent :type Primitive%20Component%20Object%20Reference) (OtherActor :type Actor%20Object%20Reference) (OtherComp :type Primitive%20Component%20Object%20Reference) (OtherBodyIndex :type Integer) (bFromSweep :type Boolean) (SweepResult :type Hit%20Result%20Structure%20%28by%20ref%29)))

(event OnComponentEndOverlap(Box)
  (params (OverlappedComponent :type Primitive%20Component%20Object%20Reference) (OtherActor :type Actor%20Object%20Reference) (OtherComp :type Primitive%20Component%20Object%20Reference) (OtherBodyIndex :type Integer)))

(event Interacted(BP_Interacred)
  ;[1 1 1] На кнопку E мы вызываем удаляем наш актор, при этом действие это записывается в Pickup event который в референсе, дубликате этого актора запускает последующую логику
  (CallFunction|Pickup)
  (Development|PrintString "pickup")
  (Actor|DestroyActor))

(event Custom|Pickup
  ;[1 1 1] На кнопку E мы вызываем удаляем наш актор, при этом действие это записывается в Pickup event который в референсе, дубликате этого актора запускает последующую логику
)

(event Input|KeyboardEvents|E
  (params (Key :type Key%20Structure :default "None")))

(fn ConstructionScript)