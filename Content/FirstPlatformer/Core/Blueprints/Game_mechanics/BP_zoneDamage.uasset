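; BP_zoneDamage is a box-triggered zone that repeatedly damages a BP_PlatformerCharacter inside it.
; Begin overlap damages the character's BPCHealth and prints the amount, then loops on a half-second Delay, spawning an emitter at player 0 before each repeat.
; The loop stops at zero health or when any end overlap clears ContolZone.
; Walk-speed change nodes are present but never run.
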(event OnComponentBeginOverlap(Box)
  (params (OverlappedComponent :type Primitive%20Component%20Object%20Reference) (OtherActor :type Actor%20Object%20Reference) (OtherComp :type Primitive%20Component%20Object%20Reference) (OtherBodyIndex :type Integer) (bFromSweep :type Boolean) (SweepResult :type Hit%20Result%20Structure%20%28by%20ref%29))
  (bind _damage (Variables|Default|GetDamage))
  (Variables|Default|SetcontolZone true)
  (bind _asbp_platformer_character (Utilities|Casting|CastToBP_PlatformerCharacter OtherActor))
  (Default|Damage (Variables|/Game/FirstPlatformer/Core/Blueprints/BP_PlatformerCharacter.BP_PlatformerCharacter_C|GetBPC_health _asbp_platformer_character) _damage :!label _label)
  (Development|PrintString (Utilities|String|ToString(Float) _damage) true true "(R=1.000000,G=0.069411,B=0.000000,A=1.000000)")
  (Utilities|FlowControl|Delay 0.5)
  (if (Variables|Default|GetcontolZone)
    (if (not (== (Default|CurrentHealth (Variables|/Game/FirstPlatformer/Core/Blueprints/BP_PlatformerCharacter.BP_PlatformerCharacter_C|GetBPC_health _asbp_platformer_character)) 0.0))
      (Effects|SpawnEmitteratLocation 0 (Transformation|GetActorLocation (Game|GetPlayerCharacter 0)))
      (goto _label))))

(event OnComponentEndOverlap(Box)
  (params (OverlappedComponent :type Primitive%20Component%20Object%20Reference) (OtherActor :type Actor%20Object%20Reference) (OtherComp :type Primitive%20Component%20Object%20Reference) (OtherBodyIndex :type Integer))
  (Variables|Default|SetcontolZone false))

(fn ConstructionScript)