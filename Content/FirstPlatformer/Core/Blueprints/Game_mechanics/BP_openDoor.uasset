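; Keycard-locked swinging door that the platformer character opens and closes with E while inside its Box trigger, which toggles input.
; E or the Activ event requires a keycard and spends one on every toggle, closing included.
; The OpenDoor timeline yaws the Scene component 90 degrees, choosing direction by a dot product so it depends on the player's side.
; Closing reverses the timeline; Activate and Deactivate are stubs returning false.
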(event OnComponentBeginOverlap(Box)
  (params (OverlappedComponent :type Primitive%20Component%20Object%20Reference) (OtherActor :type Actor%20Object%20Reference) (OtherComp :type Primitive%20Component%20Object%20Reference) (OtherBodyIndex :type Integer) (bFromSweep :type Boolean) (SweepResult :type Hit%20Result%20Structure%20%28by%20ref%29))
  (Utilities|Casting|CastToBP_PlatformerCharacter OtherActor)
  (Input|EnableInput (Game|GetPlayerController 0)))

(event OnComponentEndOverlap(Box)
  (params (OverlappedComponent :type Primitive%20Component%20Object%20Reference) (OtherActor :type Actor%20Object%20Reference) (OtherComp :type Primitive%20Component%20Object%20Reference) (OtherBodyIndex :type Integer))
  (Utilities|Casting|CastToBP_PlatformerCharacter OtherActor)
  (Input|DisableInput (Game|GetPlayerController 0)))

(event Custom|OpenDoor)

(event EventBeginPlay
  (bind _asbp_platformer_character (Utilities|Casting|CastToBP_PlatformerCharacter (Game|GetPlayerCharacter 0))))

(event EventActiv
  (bind _defaultsceneroot (Variables|Default|GetDefaultSceneRoot))
  ;[1 1 1] Узнаю сколько элементов собранно, если больше 0 тогда мы открываем дверь и сразу вычитаем -1 когда открыли дверь
  (if (> (Variables|/Game/FirstPlatformer/Core/Blueprints/BP_PlatformerCharacter.BP_PlatformerCharacter_C|GetpickUpKeyCard (stale EventBeginPlay _asbp_platformer_character)) 0)
    (Variables|/Game/FirstPlatformer/Core/Blueprints/BP_PlatformerCharacter.BP_PlatformerCharacter_C|SetpickUpKeyCard (stale EventBeginPlay _asbp_platformer_character) (- (Variables|/Game/FirstPlatformer/Core/Blueprints/BP_PlatformerCharacter.BP_PlatformerCharacter_C|GetpickUpKeyCard (stale EventBeginPlay _asbp_platformer_character)) 1))
    (if (Variables|Default|GetisDoorCloset)
      (Variables|Default|SetisDoorCloset false)
      (Variables|Default|SetDot%20produkt (Math|Vector|DotProduct (Math|Vector|Normalize (- (Transformation|GetWorldLocation _defaultsceneroot) (Transformation|GetActorLocation (stale EventBeginPlay _asbp_platformer_character)))) (Math|Vector|GetForwardVector _defaultsceneroot)))
      (bind (_direction _newtrack_0) (Timeline|open%20door Play)
        (:Update
          (Transformation|SetRelativeRotation (Variables|Default|GetScene) (Math|Rotator|MakeRotator 0.0 0.0 (Math|Float|Lerp 0.0 (Math|Float|SelectFloat 9e+01 -9e+01 (>= (Variables|Default|GetDot%20produkt) 0.0)) _newtrack_0)) false false))
        (:Finished
          (switch Utilities|FlowControl|Switch|SwitchonETimelineDirection _direction
            (:Backward
              (Variables|Default|SetisDoorCloset true)))))
      (else
        (Timeline|open%20door Reverse)))))

(event Input|KeyboardEvents|E
  (params (Key :type Key%20Structure :default "None"))
  (bind _defaultsceneroot (Variables|Default|GetDefaultSceneRoot))
  (:Pressed
    ;[1 1 1] Узнаю сколько элементов собранно, если больше 0 тогда мы открываем дверь и сразу вычитаем -1 когда открыли дверь
    (if (> (Variables|/Game/FirstPlatformer/Core/Blueprints/BP_PlatformerCharacter.BP_PlatformerCharacter_C|GetpickUpKeyCard (stale EventBeginPlay _asbp_platformer_character)) 0)
      (Variables|/Game/FirstPlatformer/Core/Blueprints/BP_PlatformerCharacter.BP_PlatformerCharacter_C|SetpickUpKeyCard (stale EventBeginPlay _asbp_platformer_character) (- (Variables|/Game/FirstPlatformer/Core/Blueprints/BP_PlatformerCharacter.BP_PlatformerCharacter_C|GetpickUpKeyCard (stale EventBeginPlay _asbp_platformer_character)) 1))
      (if (Variables|Default|GetisDoorCloset)
        (Variables|Default|SetisDoorCloset false)
        (Variables|Default|SetDot%20produkt (Math|Vector|DotProduct (Math|Vector|Normalize (- (Transformation|GetWorldLocation _defaultsceneroot) (Transformation|GetActorLocation (stale EventBeginPlay _asbp_platformer_character)))) (Math|Vector|GetForwardVector _defaultsceneroot)))
        (bind (_direction _newtrack_0) (Timeline|open%20door Play)
          (:Update
            (Transformation|SetRelativeRotation (Variables|Default|GetScene) (Math|Rotator|MakeRotator 0.0 0.0 (Math|Float|Lerp 0.0 (Math|Float|SelectFloat 9e+01 -9e+01 (>= (Variables|Default|GetDot%20produkt) 0.0)) _newtrack_0)) false false))
          (:Finished
            (switch Utilities|FlowControl|Switch|SwitchonETimelineDirection _direction
              (:Backward
                (Variables|Default|SetisDoorCloset true)))))
        (else
          (Timeline|open%20door Reverse))))))

(fn ConstructionScript)

(fn Activate
  (return false))

(fn Deactivate
  (return false))