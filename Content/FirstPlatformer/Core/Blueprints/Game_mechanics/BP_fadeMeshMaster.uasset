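; Mesh actor that fades its opacity down to a configurable amount and back through StartFade and EndFade events.
; The construction script applies the chosen mesh, and StartFade swaps material slot 0 to a dynamic instance of a fade material.
; A timeline drives the Opacity parameter, playing forward to fade and reversing to recover.
; Whenever the computed opacity equals 1, the update restores the mesh's original material.
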(event EventEndFade
  (bind _newtrack_0 (Timeline|FadeMesh Reverse)
    (:Update
      (Rendering|Material|SetScalarParameterValue (Variables|Default|GetDynamicMaterial) "Opacity" (- 1.0 (* _newtrack_0 (- 1.0 (Variables|Default|GetEndingFadeAmount)))) :!class /Script/Engine.MaterialInstanceDynamic)
      (if (== (- 1.0 (* _newtrack_0 (- 1.0 (Variables|Default|GetEndingFadeAmount)))) 1.0)
        (Rendering|Material|SetMaterial (Variables|Default|GetStaticMesh) 0 (Rendering|Material|GetMaterial (Variables|Default|GetMeshToUse) 0))))))

(event EventStartFade
  (CallFunction|FadeMaterialSwitch)
  (bind _newtrack_0 (Timeline|FadeMesh Play)
    (:Update
      (Rendering|Material|SetScalarParameterValue (Variables|Default|GetDynamicMaterial) "Opacity" (- 1.0 (* _newtrack_0 (- 1.0 (Variables|Default|GetEndingFadeAmount)))) :!class /Script/Engine.MaterialInstanceDynamic)
      (if (== (- 1.0 (* _newtrack_0 (- 1.0 (Variables|Default|GetEndingFadeAmount)))) 1.0)
        (Rendering|Material|SetMaterial (Variables|Default|GetStaticMesh) 0 (Rendering|Material|GetMaterial (Variables|Default|GetMeshToUse) 0))))))

(fn ConstructionScript
  (Components|StaticMesh|SetStaticMesh (Variables|Default|GetStaticMesh) (Variables|Default|GetMeshToUse)))

(fn FadeMaterialSwitch
  (bind _returnvalue (Rendering|Material|CreateDynamicMaterialInstance (Variables|Default|GetFadeMaterial) "None" "None" :!class /Script/Engine.KismetMaterialLibrary))
  (bind _output_get (Variables|Default|SetDynamicMaterial _returnvalue))
  (Rendering|Material|SetMaterial (Variables|Default|GetStaticMesh) 0 _output_get))