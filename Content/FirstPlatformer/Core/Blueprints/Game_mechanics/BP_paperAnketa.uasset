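; BP_paperAnketa is an interactable paper actor that shows the WB_paperAnketa widget and is destroyed after reading.
; A Box overlap with BP_PlatformerCharacter enables the actor's input and reveals an E prompt, both reversed on exit.
; Pressing E alternates via FlipFlop between opening the widget with look and move input ignored, and removing it, restoring input and destroying the actor.
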(event OnComponentBeginOverlap(Box)
  (params (OverlappedComponent :type Primitive%20Component%20Object%20Reference) (OtherActor :type Actor%20Object%20Reference) (OtherComp :type Primitive%20Component%20Object%20Reference) (OtherBodyIndex :type Integer) (bFromSweep :type Boolean) (SweepResult :type Hit%20Result%20Structure%20%28by%20ref%29))
  (Utilities|Casting|CastToBP_PlatformerCharacter OtherActor)
  (Input|EnableInput (Game|GetPlayerController 0))
  (Development|SetHiddeninGame (Variables|Default|GetE) false false))

(event OnComponentEndOverlap(Box)
  (params (OverlappedComponent :type Primitive%20Component%20Object%20Reference) (OtherActor :type Actor%20Object%20Reference) (OtherComp :type Primitive%20Component%20Object%20Reference) (OtherBodyIndex :type Integer))
  (Utilities|Casting|CastToBP_PlatformerCharacter OtherActor)
  (Input|DisableInput (Game|GetPlayerController 0))
  (Development|SetHiddeninGame (Variables|Default|GetE) true false))

(event Input|KeyboardEvents|E
  (params (Key :type Key%20Structure :default "None"))
  (bind _returnvalue (Game|GetPlayerController 0))
  (:Pressed
    (Utilities|FlowControl|FlipFlop
      (:A
        (bind _returnvalue_2 (Game|ConstructObjectfromClass "/Game/FirstPlatformer/Core/UI/WB_paperAnketa.WB_paperAnketa_C"))
        (UserInterface|Viewport|AddtoViewport _returnvalue_2 0)
        (Input|SetIgnoreLookInput _returnvalue true)
        (Input|SetIgnoreMoveInput _returnvalue true))
      (:B
        (Widget|RemovefromParent _returnvalue_2)
        (Input|SetIgnoreLookInput _returnvalue false)
        (Input|SetIgnoreMoveInput _returnvalue false)
        (Actor|DestroyActor)))))

(fn ConstructionScript)