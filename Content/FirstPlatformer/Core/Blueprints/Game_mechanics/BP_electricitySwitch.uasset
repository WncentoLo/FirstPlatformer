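; BP_electricitySwitch is an interactive switch that activates or deactivates a referenced target actor, ActorToActiv.
; Box overlap enables input only while BP_PlatformerCharacter is inside, letting E operate it.
; Each press sends an activate or deactivate interface message plus ActivMessage to the target, then plays or reverses the PushButton timeline.
; The timeline lerps the button between off and on positions and derives the ControlSwitcher toggle state from its alpha.
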(event OnComponentBeginOverlap(Box)
  (params (OverlappedComponent :type Primitive%20Component%20Object%20Reference) (OtherActor :type Actor%20Object%20Reference) (OtherComp :type Primitive%20Component%20Object%20Reference) (OtherBodyIndex :type Integer) (bFromSweep :type Boolean) (SweepResult :type Hit%20Result%20Structure%20%28by%20ref%29))
  ;[1 1 1] Проверка находится ли наш персонаж внутри collision Box
  (Utilities|Casting|CastToBP_PlatformerCharacter OtherActor)
  (Input|EnableInput (Game|GetPlayerController 0)))

(event OnComponentEndOverlap(Box)
  (params (OverlappedComponent :type Primitive%20Component%20Object%20Reference) (OtherActor :type Actor%20Object%20Reference) (OtherComp :type Primitive%20Component%20Object%20Reference) (OtherBodyIndex :type Integer))
  ;[1 1 1] Проверка находится ли наш персонаж внутри collision Box
  (Utilities|Casting|CastToBP_PlatformerCharacter OtherActor)
  (Input|DisableInput (Game|GetPlayerController 0)))

(event Input|KeyboardEvents|E
  (params (Key :type Key%20Structure :default "None"))
  (bind _actor_to_activ (Variables|Default|GetActor%20to%20activ))
  (:Pressed
    (bind _output_get (Variables|Default|SetcontrolSwitcher (Variables|Default|GetcontrolSwitcher)))
    (if _output_get
      ;[1 1 1] Интерфейс с настройками внутри BP в функции
      (Class|BPIActivation|Activate(Message) _actor_to_activ)
      ;[1 1 1] Вызовы через Event другого Интерфейса с запуском настроеной функции
      (Class|BPIComunication|Activ(Message) _actor_to_activ)
      (bind _off_on_animation (Timeline|pushButton Play)
        (:Update
          (Transformation|SetRelativeLocation (Variables|Default|Getswitcher_button) (Math|Vector|Lerp(Vector) (Variables|Default|GetoffPosition) (Variables|Default|GetonPosition) _off_on_animation) false false)
          (Variables|Default|SetcontrolSwitcher (< _off_on_animation 1.0))))
      (else
        (Class|BPIActivation|Deactivate(Message) _actor_to_activ)
        (Class|BPIComunication|Activ(Message) _actor_to_activ)
        (Timeline|pushButton Reverse)))))

(fn ConstructionScript)

(fn Activate
  (return true))

(fn Deactivate
  (return true))