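; Actor component that shows the owning actor's text render component while something overlaps that actor, and hides it when the overlap ends.
; On BeginPlay it binds to the owner's begin and end overlap events.
; Each handler looks up the owner's TextRenderComponent by class and toggles its hidden-in-game state, without checking which actor triggered the overlap.
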(event Custom|OnActorBeginOverlap_Event
  (params (OverlappedActor :type Actor%20Object%20Reference) (OtherActor :type Actor%20Object%20Reference))
  (Development|SetHiddeninGame (Actor|GetComponentbyClass (Components|GetOwner) "/Script/Engine.TextRenderComponent") false false))

(event Custom|OnActorendOverlap_Event
  (params (OverlappedActor :type Actor%20Object%20Reference) (OtherActor :type Actor%20Object%20Reference))
  (Development|SetHiddeninGame (Actor|GetComponentbyClass (Components|GetOwner) "/Script/Engine.TextRenderComponent") true false))

(event EventBeginPlay
  (bind _returnvalue (Components|GetOwner))
  (EventDispatchers|AssignOnActorBeginOverlap _returnvalue (delegate Custom|OnActorBeginOverlap_Event))
  (Collision|BindEventtoOnActorEndOverlap _returnvalue (delegate Custom|OnActorendOverlap_Event)))