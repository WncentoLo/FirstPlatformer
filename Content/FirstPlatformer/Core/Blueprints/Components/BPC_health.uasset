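; BPC_health is a health component that tracks current and maximum health for its owner.
; It fills Health on BeginPlay, offers clamped healing, damage and full recovery, and exposes current health as a value or fraction of maximum.
; EDChange announces changes, though Damage fires it before subtracting, so listeners reading Health then get the old value.
; Reaching zero fires EDDeath through a DoOnce, which Recovery does not reset.
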(event EventBeginPlay
  (CallFunction|Recovery)
  (Default|CallEDChange))

(fn CurrentHealth
  (return (Variables|Default|GetHealth)))

(fn GetPersonHealth
  (return (/ (Variables|Default|GetHealth) (Variables|Default|GetMaxHealth))))

(fn AddHealth
  (params (Add :type Float%20%28double-precision%29))
  (Variables|Default|SetHealth (Math|Float|Min(Float) (+ Add (Variables|Default|GetHealth)) (Variables|Default|GetMaxHealth)))
  (Default|CallEDChange))

(fn Damage
  (params (Damage :type Float%20%28double-precision%29))
  (Default|CallEDChange)
  (bind _output_get (Variables|Default|SetHealth (Math|Float|Max(Float) (- (Variables|Default|GetHealth) Damage) 0.0)))
  (if (== _output_get 0.0)
    (Utilities|FlowControl|DoOnce false
      (:Completed
        (Default|CallEDDeath)
        (return)))))

(fn Recovery
  (Variables|Default|SetHealth (Variables|Default|GetMaxHealth))
  (Default|CallEDChange))