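; BP_CameraMovements is a trigger-box actor that pulls the platformer character's camera back while the character is inside it.
; Begin overlap casts to BP_PlatformerCharacter, caches it and sets ShiftCamera; any end overlap clears the flag.
; Tick uses FInterpTo to ease the cached player's CameraBoom arm length toward the far or default distance according to that flag.
; Interp speed is scaled by delta time, so easing varies with frame rate.
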(event OnComponentBeginOverlap(Box)
  (params (OverlappedComponent :type Primitive%20Component%20Object%20Reference) (OtherActor :type Actor%20Object%20Reference) (OtherComp :type Primitive%20Component%20Object%20Reference) (OtherBodyIndex :type Integer) (bFromSweep :type Boolean) (SweepResult :type Hit%20Result%20Structure%20%28by%20ref%29))
  ;[1 1 1] Проверяем каст на нашего персонажа и записываем в переменуюю Player если он пересекается с коллизией box
  (bind _asbp_platformer_character (Utilities|Casting|CastToBP_PlatformerCharacter OtherActor))
  (Variables|Default|SetPlayer _asbp_platformer_character)
  (Variables|Default|SetbShiftCamera true))

(event OnComponentEndOverlap(Box)
  (params (OverlappedComponent :type Primitive%20Component%20Object%20Reference) (OtherActor :type Actor%20Object%20Reference) (OtherComp :type Primitive%20Component%20Object%20Reference) (OtherBodyIndex :type Integer))
  ;[1 1 1] Проверка выхода за пределы box колизии и записывание результата в булевую переменную
  (Variables|Default|SetbShiftCamera false))

(event EventTick
  (params (DeltaSeconds :type Float%20%28single-precision%29))
  (bind _returnvalue (Utilities|Time|GetWorldDeltaSeconds))
  (bind _returnvalue_2 (Utilities|Time|GetWorldDeltaSeconds))
  (bind _player (Variables|Default|GetPlayer))
  (bind _player_2 (Variables|Default|GetPlayer))
  (bind _cameraboom (Variables|/Game/FirstPlatformer/Core/Blueprints/BP_PlatformerCharacter.BP_PlatformerCharacter_C|GetCameraBoom _player_2))
  (bind _cameraboom_2 (Variables|/Game/FirstPlatformer/Core/Blueprints/BP_PlatformerCharacter.BP_PlatformerCharacter_C|GetCameraBoom _player))
  ;[1 1 1] Контроль отдаления камеры от зоны (box колизии)
  (if (Variables|Default|GetbShiftCamera)
    ;;[1 1 1] Из переменной Player достаем параметры камеры и изменяем их отдоляя на дистанцию 1400
    (Utilities|IsValid _player
      (:Is%20Valid
        (Variables|/Script/Engine.SpringArmComponent|SetTargetArmLength _cameraboom_2 (Math|Interpolation|FInterpTo (Variables|/Script/Engine.SpringArmComponent|GetTargetArmLength _cameraboom_2) 1.6e+03 _returnvalue_2 (* _returnvalue_2 5e+01)))))
    (else
      ;;[1 1 1] Возвращает камеру в прежднее положение
      (Utilities|IsValid _player_2
        (:Is%20Valid
          (Variables|/Script/Engine.SpringArmComponent|SetTargetArmLength _cameraboom (Math|Interpolation|FInterpTo (Variables|/Script/Engine.SpringArmComponent|GetTargetArmLength _cameraboom) 1.2e+03 _returnvalue (* _returnvalue 5e+01))))))))

(fn ConstructionScript)